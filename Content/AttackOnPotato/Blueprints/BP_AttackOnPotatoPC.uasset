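; Player controller for Attack On Potato that makes in-world 3D buttons clickable with the mouse.
; A left click traces under the cursor on the Visibility channel and acts on the hit 3DButton's type.
; Restart and Menu fade the camera out, show a loading-screen widget, then open the game level or title menu after short delays.
; Close exits the game through a console command.
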(event `Key|LeftMouseButton` :consume false
  (params (Key :type "Key Structure" :default "AnyKey"))
  (:`Pressed`
    (bind _as3dbutton (cast `/Game/AttackOnPotato/Blueprints/3DButton` (`.HitActor` (`GameplayStatics.BreakHitResult` (`self.GetHitResultUnderCursorByChannel` "TraceTypeQuery1")))))
    (switch `string` (`/Game/AttackOnPotato/Blueprints/3DButton.ButtonType` _as3dbutton)
      (:`Restart`
        (`PlayerCameraManager.StartCameraFade` :`self` (`GameplayStatics.GetPlayerCameraManager` 0) :`ToAlpha` 1.0 :`Duration` 1.0)
        (`KismetSystemLibrary.Delay` 1.0)
        (bind _returnvalue (`|CreateWidget` "/Game/AttackOnPotato/UMG/WB_LoadingScreen.WB_LoadingScreen_C"))
        (`UserWidget.AddToViewport` _returnvalue 0)
        (`KismetSystemLibrary.Delay` 0.2)
        (`GameplayStatics.OpenLevel` "Game_Level"))
      (:`Close`
        (`KismetSystemLibrary.ExecuteConsoleCommand` "Exit"))
      (:`Menu`
        (`PlayerCameraManager.StartCameraFade` :`self` (`GameplayStatics.GetPlayerCameraManager` 0) :`ToAlpha` 1.0 :`Duration` 1.0)
        (`KismetSystemLibrary.Delay` 1.0)
        (bind _returnvalue_2 (`|CreateWidget` "/Game/AttackOnPotato/UMG/WB_LoadingScreen.WB_LoadingScreen_C"))
        (`UserWidget.AddToViewport` _returnvalue_2 0)
        (`KismetSystemLibrary.Delay` 0.2)
        (`GameplayStatics.OpenLevel` "Title_Menu")))))

(fn `UserConstructionScript`)