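; Enemy spawner that populates the navmesh around itself with AI characters, with a population limit that grows over time.
; A looping timer calls Spawn until SpawnCounter reaches MaxSpawn, which a Tick-driven Delay periodically raises toward MaxMaxSpawn.
; Spawn recursively retries when a random navigable point is near the player, but spawns at a separately rolled point.
; Each spawn gets random yaw and scale, and this Blueprint never decrements the counter.
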(event `CustomEvent_0`)

(event `self.ReceiveBeginPlay`
  (set `self.SpawnCounter` 0)
  (`KismetSystemLibrary.K2_SetTimer` null "Spawn" (`self.SpawnDelay`) true))

(event `self.ReceiveTick`
  (params (DeltaSeconds :type "Float (single-precision)"))
  (`KismetSystemLibrary.Delay` 10.0)
  (set `self.MaxSpawn` (`KismetMathLibrary.Clamp` (+ (`self.MaxSpawn`) 5) 0 (`self.MaxMaxSpawn`))))

(fn `Spawn`
  (bind _returnvalue (`NavigationSystem.GetRandomPointInNavigableRadius` (`self.K2_GetActorLocation`) 5000.0 (`self.NavMesh`)))
  (if (< (`self.SpawnCounter`) (`self.MaxSpawn`))
    (if (< (`KismetMathLibrary.VSize` (- _returnvalue (`self.K2_GetActorLocation` (`GameplayStatics.GetPlayerCharacter` 0)))) 500.0)
      (`self.Spawn`)
      (else
        (`|SpawnActorFromClass` "/Game/AttackOnPotato/AI/AICharacter.AICharacter_C" (`KismetMathLibrary.MakeTransform` _returnvalue (`KismetMathLibrary.MakeRotator` 0.0 0.0 (`KismetMathLibrary.RandomFloatInRange` 0.0 360.0)) (`KismetMathLibrary.Conv_DoubleToVector` (`KismetMathLibrary.RandomFloatInRange` 0.7 1.2))) "Undefined" "OverrideRootScale")
        (`/Engine/EditorBlueprintResources/StandardMacros.IncrementInt` (`self.SpawnCounter`))))))

(fn `UserConstructionScript`)