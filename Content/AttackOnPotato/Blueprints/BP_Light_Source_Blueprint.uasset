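; Sun light actor that pitches from a start angle toward an end angle over the level's duration, acting as a day-cycle timer.
; Tick passes through a short Delay, accumulates time, applies a fixed rotation step, prints the running total and refreshes the Skysphere's sun direction.
; Past the level time, it keeps pitching by delta seconds without updating the sky; the end-of-level pause logic is disconnected.
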(event `self.ReceiveBeginPlay`
  (`self.K2_AddActorLocalRotation` (`KismetMathLibrary.MakeRotator` 0.0 (`self.Start Rotation`))))

(event `self.ReceiveTick`
  (params (DeltaSeconds :type "Float (single-precision)"))
  (bind _returnvalue (/ (/ (- (`self.End Rotation`) (`self.Start Rotation`)) (`self.Level Time`)) 100.0))
  (`KismetSystemLibrary.Delay` 0.01)
  ;[1 1 1] Timer
  (set `self.Current Time` (+ DeltaSeconds (`self.Current Time`)))
  (if (< (`self.Current Time`) (`self.Level Time`))
    (`self.K2_AddActorLocalRotation` (`KismetMathLibrary.MakeRotator` 0.0 _returnvalue))
    (bind _output_get (set `self.Rotation` (+ _returnvalue (`self.Rotation`))))
    (`KismetSystemLibrary.PrintString` (`KismetStringLibrary.Conv_DoubleToString` _output_get))
    (`/Engine/EngineSky/BP_Sky_Sphere.UpdateSunDirection` (`self.Skysphere`))
    (else
      (`self.K2_AddActorLocalRotation` (`KismetMathLibrary.MakeRotator` 0.0 DeltaSeconds)))))

(fn `UserConstructionScript`
  (`/Engine/EngineSky/BP_Sky_Sphere.UpdateSunDirection` (`self.Skysphere`)))